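; Health potion pickup that heals the player's BP_Hero by a fixed amount, with no clamp to max health.
; On BeginPlay it caches the hero and starts a timeline that animates the sprite's relative location.
; Any sphere overlap while the hero is below max health triggers a one-time heal and health-change notification, without checking the overlapping actor.
; A second timeline then moves the sprite, and the potion destroys itself after a short delay.
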(event `self.ReceiveBeginPlay`
  (bind _asbp_hero (cast `/Game/Blueprints/Hero/BP_Hero` (`GameplayStatics.GetPlayerCharacter` 0)))
  (set `self.As BP Hero` _asbp_hero)
  (bind (_direction _newtrack_1) (`Timeline|Moving`)
    (:`Update`
      (`SceneComponent.K2_SetRelativeLocation` (`self.PaperSprite`) _newtrack_1 false false))))

(event `self.Sphere.OnComponentBeginOverlap`
  (params (OverlappedComponent :type "PrimitiveComponent Object Reference") (OtherActor :type "Actor Object Reference") (OtherComp :type "PrimitiveComponent Object Reference") (OtherBodyIndex :type Integer) (bFromSweep :type Boolean) (SweepResult :type "HitResult Structure (by ref)"))
  (bind _as_bp_hero (`self.As BP Hero`))
  (bind _as_bp_hero_2 (`self.As BP Hero`))
  (bind _as_bp_hero_3 (`self.As BP Hero`))
  (if (not (>= (`/Game/Blueprints/Hero/BP_Hero.Health` _as_bp_hero_3) (`/Game/Blueprints/Hero/BP_Hero.MAX Health` _as_bp_hero_3)))
    (`/Engine/EditorBlueprintResources/StandardMacros.DoOnce` false
      (:`Completed`
        (set `/Game/Blueprints/Hero/BP_Hero.Health` (+ (`/Game/Blueprints/Hero/BP_Hero.Health` _as_bp_hero) 20.0) _as_bp_hero)
        (`/Game/Blueprints/Hero/BP_Hero.Changing Health` _as_bp_hero (/ (`/Game/Blueprints/Hero/BP_Hero.Health` _as_bp_hero_2) (`/Game/Blueprints/Hero/BP_Hero.MAX Health` _as_bp_hero_2)))
        (bind (_direction _newtrack_0) (`Timeline|Moving Up`)
          (:`Update`
            (`SceneComponent.K2_SetRelativeLocation` (`self.PaperSprite`) _newtrack_0 false false)
            (`KismetSystemLibrary.Delay` 0.4)
            (`self.K2_DestroyActor`)))))))

(fn `UserConstructionScript`)